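; Player actor for a rhythm game that moves along a clamped Y axis with the mouse and runs note play.
; BeginPlay loads a hardcoded JSON chart and starts music after a delay; Tick spawns notes ahead of their start times.
; Touch, tap (keys/buttons) and flick (accumulated mouse X) notes are judged by timing and player position, with positioned hit sounds.
; Escape pauses through time dilation, paused music and a menu widget.
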(event Custom|OnClickContinue
  (CallFunction|OnContinue))

(event EventBeginPlay
  (bind _waitingforspawn (Variables|Default|GetWaitingForSpawn))
  (bind _waitingforspawn_2 (Variables|Default|GetWaitingForSpawn))
  (bind _pausemenu (Variables|Default|GetPauseMenu))
  (bind _returnvalue (Utilities|Array|LastIndex _waitingforspawn_2))
  (bind _output (Utilities|Array|Get(acopy) _waitingforspawn_2 _returnvalue))
  (bind (_starttime _y _notetype _direction) (Utilities|Struct|BreakNoteData _output))
  (Utilities|FlowControl|Sequence
    (:then_0
      (UserInterface|Viewport|AddtoViewport _pausemenu 0)
      (Widget|SetVisibility (Variables|Default|GetPauseMenu) "Collapsed")
      (Variables|/Game/Custom/Blueprints/PauseMenu.PauseMenu_C|SetBocchi _pausemenu self)
      (EventDispatchers|BindEventtoOnClickContinue _pausemenu (delegate Custom|OnClickContinue)))
    (:then_1
      (bind _returnvalue_2 (AddComponent|AddAudioComponent false))
      (bind _output_get (Variables|Default|SetMusic _returnvalue_2))
      (Audio|Components|Audio|Stop _output_get)
      (Audio|Components|Audio|SetVolumeMultiplier _output_get (Variables|Default|GetMusicVolume) :!class /Script/Engine.AudioComponent))
    (:then_2
      ;[1 1 1] Load From Json
      (bind _returnvalue_3 (Class|EasyJsonParseManager|LoadfromFile "Levels\\Korogaru Iwa, Kimi ni Asa ga Furu\\level2.json" false)
        (:Successed
          (bind _returnvalue_4 (Class|EasyJsonObject|ReadObjects _returnvalue_3 "notes")
            (:Found
              (for _array_element _returnvalue_4
                (switch int (Class|EasyJsonObject|ReadInt _array_element "type")
                  (:Default
                    (Utilities|Array|Add _waitingforspawn_2 (Utilities|Struct|MakeNoteData (Class|EasyJsonObject|ReadFloat _array_element "startTime" 0.0) (Class|EasyJsonObject|ReadFloat _array_element "y" 0.0)) :!label _label))
                  (:0
                    (goto _label))
                  (:1
                    (Utilities|Array|Add _waitingforspawn_2 (Utilities|Struct|MakeNoteData (Class|EasyJsonObject|ReadFloat _array_element "startTime" 0.0) (Class|EasyJsonObject|ReadFloat _array_element "y" 0.0) "NewEnumerator1" (Class|EasyJsonObject|ReadInt _array_element "direction"))))
                  (:2
                    (Utilities|Array|Add _waitingforspawn_2 (Utilities|Struct|MakeNoteData (Class|EasyJsonObject|ReadFloat _array_element "startTime" 0.0) (Class|EasyJsonObject|ReadFloat _array_element "y" 0.0) "NewEnumerator2" (Class|EasyJsonObject|ReadInt _array_element "direction"))))))
              ;[1 1 1] Copy To Array
              (Utilities|Array|SetArrayElem _waitingforspawn_2 _returnvalue (Utilities|Struct|MakeNoteData _starttime _y _notetype _direction true))
              (for (_ _array_index) _waitingforspawn
                (Utilities|Array|Add (Variables|Default|GetCopyOfNoteData) (Utilities|Array|Get(acopy) _waitingforspawn _array_index))))
            (:NotFound
              (Development|PrintString "Failed To Load" :!label _label_2))))
        (:Failed
          (goto _label_2))))
    (:then_3
      (Variables|Default|SetisPlaying true)
      (Variables|Default|SetStartTime (+ (Utilities|Time|GetTimeSeconds) 2.5))
      (Audio|Components|Audio|Stop (Variables|Default|GetMusic))
      (Utilities|FlowControl|Delay 2.5)
      (Audio|Components|Audio|Play (Variables|Default|GetMusic) 0.0)
      (Variables|Default|SetcanPause true))))

(event EventTick
  (params (DeltaSeconds :type Float%20%28single-precision%29))
  (bind _returnvalue (Game|GetPlayerController 0))
  (bind _returnvalue_2 (Math|Transform|MakeTransform "70.000000,320.000000,-150.000000"))
  (bind _returnvalue_3 (Game|GetPlayerController 0))
  (bind _returnvalue_4 (Game|GetPlayerController 0))
  (bind _judge (Variables|Default|GetJudge))
  (bind _waitingforspawn (Variables|Default|GetWaitingForSpawn))
  (bind _spawnedflicknoteobject (Variables|Default|GetSpawnedFlickNoteObject))
  (bind _judgecorrection (Variables|Default|GetJudgeCorrection))
  (bind _pausemenu (Variables|Default|GetPauseMenu))
  (bind _spawnedtapnoteobject (Variables|Default|GetSpawnedTapNoteObject))
  (bind _judgecorrection_2 (Variables|Default|GetJudgeCorrection))
  (bind _spawnedtouchnoteobject (Variables|Default|GetSpawnedTouchNoteObject))
  (bind _deltax (Class|PlayerController|GetInputMouseDelta _returnvalue_4))
  (bind _returnvalue_5 (Transformation|GetWorldLocation _judge))
  (bind _returnvalue_6 (> _deltax 0.0))
  (bind _returnvalue_7 (> 0.0 _deltax))
  (bind (_x _y _z) (Math|Vector|BreakVector _returnvalue_5))
  (Utilities|FlowControl|Sequence
    (:then_0
      (if (Game|Player|WasInputKeyJustPressed _returnvalue_3 "Escape")
        ;[1 1 1] Set Pause State
        (if (Variables|Default|GetcanPause)
          (if (not (Variables|Default|GetisPausing))
            (Variables|Default|SetisPlaying false)
            (Utilities|Time|SetGlobalTimeDilation 0.0)
            (Variables|Default|SetisPausing true)
            (Widget|SetVisibility (Variables|Default|GetPauseMenu) "Visible")
            (Class|AudioComponent|SetPaused (Variables|Default|GetMusic) true)
            (UserInterface|Animation|PlayAnimation _pausemenu (Variables|/Game/Custom/Blueprints/PauseMenu.PauseMenu_C|GetShow _pausemenu) 0.0 1 "Forward" 1.0 true)
            (Variables|/Script/Engine.PlayerController|SetbShowMouseCursor _returnvalue_3 true)))))
    (:then_1
      (if (Variables|Default|GetisPlaying)
        ;[1 1 1] Control Bocchi
        (|Move)
        (Math|Float|Clamp(Float))
        ;[1 1 1] Note Spawn
        (bind _array_element (Utilities|Array|ForEachLoopwithBreak _waitingforspawn :!label _label)
          (:LoopBody
            (bind _time (CallFunction|GetGameTime))
            (if (>= _time (- (.StartTime (Utilities|Struct|BreakNoteData _array_element)) (Variables|Default|GetDuration)))
              (switch Utilities|FlowControl|Switch|SwitchonNoteType (.NoteType (Utilities|Struct|BreakNoteData _array_element))
                (:NewEnumerator0
                  (bind _returnvalue_8 (Game|SpawnActorfromClass "/Game/Custom/Blueprints/NoteObject_Touch.NoteObject_Touch_C" _returnvalue_2 "Undefined" 0 0))
                  (Variables|/Game/Custom/Blueprints/NoteObject.NoteObject_C|SetNoteData _returnvalue_8 _array_element)
                  (Variables|/Game/Custom/Blueprints/NoteObject.NoteObject_C|SetBocchi _returnvalue_8 self)
                  (Default|SetArrowDirection _returnvalue_8)
                  (Utilities|Array|Add (Variables|Default|GetSpawnedTouchNoteObject) _returnvalue_8)
                  (Utilities|Array|RemoveItem _waitingforspawn _array_element))
                (:NewEnumerator1
                  (bind _returnvalue_9 (Game|SpawnActorfromClass "/Game/Custom/Blueprints/NoteObject_Tap.NoteObject_Tap_C" _returnvalue_2 "Undefined" 0 0))
                  (Variables|/Game/Custom/Blueprints/NoteObject.NoteObject_C|SetNoteData _returnvalue_9 _array_element)
                  (Variables|/Game/Custom/Blueprints/NoteObject.NoteObject_C|SetBocchi _returnvalue_9 self)
                  (Default|SetArrowDirection _returnvalue_9)
                  (Utilities|Array|Add (Variables|Default|GetSpawnedTapNoteObject) _returnvalue_9)
                  (Utilities|Array|RemoveItem _waitingforspawn _array_element))
                (:NewEnumerator2
                  (bind _returnvalue_10 (Game|SpawnActorfromClass "/Game/Custom/Blueprints/NoteObject_Flick.NoteObject_Flick_C" _returnvalue_2 "Undefined" 0 0))
                  (Variables|/Game/Custom/Blueprints/NoteObject.NoteObject_C|SetNoteData _returnvalue_10 _array_element)
                  (Variables|/Game/Custom/Blueprints/NoteObject.NoteObject_C|SetBocchi _returnvalue_10 self)
                  (Default|SetArrowDirection _returnvalue_10)
                  (Utilities|Array|Add (Variables|Default|GetSpawnedFlickNoteObject) _returnvalue_10)
                  (Utilities|Array|RemoveItem _waitingforspawn _array_element)))
              (else
                (goto _label Break))))
          (:Completed
            ;[1 1 1] Touch Note Judgement
            (bind (_array_element_2 _array_index) (Utilities|Array|ForEachLoopwithBreak _spawnedtouchnoteobject :!label _label_2)
              (:LoopBody
                (bind _time_2 (CallFunction|GetGameTime))
                (if (>= _time_2 (.StartTime (Utilities|Struct|BreakNoteData (Variables|/Game/Custom/Blueprints/NoteObject.NoteObject_C|GetNoteData _array_element_2))))
                  (bind _result (CallFunction|IsPositionAcceptable (.Y (Utilities|Struct|BreakNoteData (Variables|/Game/Custom/Blueprints/NoteObject.NoteObject_C|GetNoteData _array_element_2)))))
                  (if (>= _time_2 (+ (.StartTime (Utilities|Struct|BreakNoteData (Variables|/Game/Custom/Blueprints/NoteObject.NoteObject_C|GetNoteData _array_element_2))) (Variables|Default|GetJudgeCorrection)))
                    (if _result
                      (Development|PrintString "Clear" false :!label _label_3)
                      (Variables|Default|SetNoteCleared true)
                      (Variables|Default|SetLastHitPosition (Transformation|GetActorLocation _array_element_2))
                      (else
                        (Development|PrintString "Miss" false)))
                    (elif _result
                      (goto _label_3)
                      (else
                        (goto _label_2 Break))))
                  (Actor|DestroyActor _array_element_2)
                  (Utilities|Array|RemoveIndex _spawnedtouchnoteobject _array_index)
                  (else
                    (goto _label_2 Break))))
              (:Completed
                ;[1 1 1] Tap Note Judgement
                (bind _array_element_3 (Utilities|Array|ForEachLoopwithBreak _spawnedtapnoteobject :!label _label_4)
                  (:LoopBody
                    (if (Utilities|IsValid _array_element_3)
                      (if (not (Variables|/Game/Custom/Blueprints/NoteObject.NoteObject_C|GetIsCleared _array_element_3))
                        (bind _time_3 (CallFunction|GetGameTime))
                        (bind _result_2 (CallFunction|IsPositionAcceptable (.Y (Utilities|Struct|BreakNoteData (Variables|/Game/Custom/Blueprints/NoteObject.NoteObject_C|GetNoteData _array_element_3)))))
                        (if (and _result_2 (or (and (> (.Direction (Utilities|Struct|BreakNoteData (Variables|/Game/Custom/Blueprints/NoteObject.NoteObject_C|GetNoteData _array_element_3))) -1) (or (Game|Player|WasInputKeyJustPressed _returnvalue "S") (Game|Player|WasInputKeyJustPressed _returnvalue "RightMouseButton"))) (and (< (.Direction (Utilities|Struct|BreakNoteData (Variables|/Game/Custom/Blueprints/NoteObject.NoteObject_C|GetNoteData _array_element_3))) 0) (or (Game|Player|WasInputKeyJustPressed _returnvalue "A") (Game|Player|WasInputKeyJustPressed _returnvalue "LeftMouseButton")))))
                          (if (and (>= _time_3 (- (.StartTime (Utilities|Struct|BreakNoteData (Variables|/Game/Custom/Blueprints/NoteObject.NoteObject_C|GetNoteData _array_element_3))) _judgecorrection_2)) (>= (+ _judgecorrection_2 (.StartTime (Utilities|Struct|BreakNoteData (Variables|/Game/Custom/Blueprints/NoteObject.NoteObject_C|GetNoteData _array_element_3)))) _time_3))
                            (Development|PrintString "Clear" false false)
                            (Variables|Default|SetNoteCleared true)
                            (Variables|Default|SetLastHitPosition (Transformation|GetActorLocation _array_element_3))
                            (Development|PrintString (Utilities|String|ToString(Float) (.StartTime (Utilities|Struct|BreakNoteData (Variables|/Game/Custom/Blueprints/NoteObject.NoteObject_C|GetNoteData _array_element_3)))) false false)
                            (Variables|/Game/Custom/Blueprints/NoteObject.NoteObject_C|SetIsCleared _array_element_3 true :!label _label_5)
                            (Actor|DestroyActor _array_element_3)
                            (Utilities|Array|RemoveItem _spawnedtapnoteobject _array_element_3)
                            (goto _label_4 Break)
                            (else
                              (if (> _time_3 (+ _judgecorrection_2 (.StartTime (Utilities|Struct|BreakNoteData (Variables|/Game/Custom/Blueprints/NoteObject.NoteObject_C|GetNoteData _array_element_3))))) :!label _label_6
                                (Development|PrintString "Miss" false false)
                                (goto _label_5))))
                          (else
                            (goto _label_6))))))
                  (:Completed
                    ;[1 1 1] Mouse X Movement Add System
                    (if (== _deltax 0.0)
                      (Variables|Default|SetMovedMousePositionX 0.0)
                      (elif (or (and _returnvalue_6 (> (Variables|Default|GetMovedMousePositionX) 0.0)) (and _returnvalue_7 (> 0.0 (Variables|Default|GetMovedMousePositionX))))
                        (Variables|Default|SetMovedMousePositionX (+ _deltax (Variables|Default|GetMovedMousePositionX)) :!label _label_7)
                        (elif (== (Variables|Default|GetMovedMousePositionX) 0.0)
                          (goto _label_7)
                          (elif (or (and _returnvalue_6 (> 0.0 (Variables|Default|GetMovedMousePositionX))) (and _returnvalue_7 (> (Variables|Default|GetMovedMousePositionX) 0.0)))
                            (Variables|Default|SetMovedMousePositionX _deltax)
                            (elif (or (and _returnvalue_6 (== (Variables|Default|GetMovedMousePositionX) 0.0)) (and _returnvalue_7 (== (Variables|Default|GetMovedMousePositionX) 0.0)))
                              (Variables|Default|SetMovedMousePositionX _deltax))))))
                    ;[1 1 1] Tap Note Judgement
                    (bind _array_element_4 (Utilities|Array|ForEachLoopwithBreak _spawnedflicknoteobject :!label _label_8)
                      (:LoopBody
                        (if (Utilities|IsValid _array_element_4)
                          (if (not (Variables|/Game/Custom/Blueprints/NoteObject.NoteObject_C|GetIsCleared _array_element_4))
                            (bind _time_4 (CallFunction|GetGameTime))
                            (bind _result_3 (CallFunction|IsPositionAcceptable (.Y (Utilities|Struct|BreakNoteData (Variables|/Game/Custom/Blueprints/NoteObject.NoteObject_C|GetNoteData _array_element_4)))))
                            (if (and _result_3 (or (Math|Boolean|ANDBoolean (> (.Direction (Utilities|Struct|BreakNoteData (Variables|/Game/Custom/Blueprints/NoteObject.NoteObject_C|GetNoteData _array_element_4))) -1) (> (Variables|Default|GetMovedMousePositionX) 0.0) (> (Math|Float|Absolute(Float) (Variables|Default|GetMovedMousePositionX)) (Variables|Default|GetFlickDragCorrection))) (Math|Boolean|ANDBoolean (< (.Direction (Utilities|Struct|BreakNoteData (Variables|/Game/Custom/Blueprints/NoteObject.NoteObject_C|GetNoteData _array_element_4))) 0) (> 0.0 (Variables|Default|GetMovedMousePositionX)) (> (Math|Float|Absolute(Float) (Variables|Default|GetMovedMousePositionX)) (Variables|Default|GetFlickDragCorrection)))))
                              (if (and (>= _time_4 (- (.StartTime (Utilities|Struct|BreakNoteData (Variables|/Game/Custom/Blueprints/NoteObject.NoteObject_C|GetNoteData _array_element_4))) _judgecorrection)) (>= (+ _judgecorrection (.StartTime (Utilities|Struct|BreakNoteData (Variables|/Game/Custom/Blueprints/NoteObject.NoteObject_C|GetNoteData _array_element_4)))) _time_4))
                                (Development|PrintString "Clear" false false)
                                (Variables|Default|SetNoteCleared true)
                                (Variables|Default|SetLastHitPosition (Transformation|GetActorLocation _array_element_4))
                                (Development|PrintString (Utilities|String|ToString(Float) (.StartTime (Utilities|Struct|BreakNoteData (Variables|/Game/Custom/Blueprints/NoteObject.NoteObject_C|GetNoteData _array_element_4)))) false false)
                                (Variables|Default|SetMovedMousePositionX 0.0)
                                (Variables|/Game/Custom/Blueprints/NoteObject.NoteObject_C|SetIsCleared _array_element_4 true :!label _label_9)
                                (Actor|DestroyActor _array_element_4)
                                (Utilities|Array|RemoveItem _spawnedflicknoteobject _array_element_4)
                                (goto _label_8 Break)
                                (else
                                  (if (> _time_4 (+ _judgecorrection (.StartTime (Utilities|Struct|BreakNoteData (Variables|/Game/Custom/Blueprints/NoteObject.NoteObject_C|GetNoteData _array_element_4))))) :!label _label_10
                                    (Development|PrintString "Miss" false false)
                                    (goto _label_9))))
                              (else
                                (goto _label_10))))))
                      (:Completed
                        ;[1 1 1] Play HitSound
                        (if (Variables|Default|GetNoteCleared)
                          (Variables|Default|SetNoteCleared false)
                          (bind _returnvalue_11 (Audio|SpawnSoundatLocation "/Game/Custom/Sounds/soft-hitclap.soft-hitclap" (Math|Vector|MakeVector _x (.Y (Math|Vector|BreakVector (Variables|Default|GetLastHitPosition))) _z) "0, 0, 0" 0.34 1.0 0.0 "/Game/Custom/Sounds/NewSoundAttenuation.NewSoundAttenuation" 0))
                          (Variables|/Script/Engine.AudioComponent|SetbAllowSpatialization _returnvalue_11 true)
                          (Variables|/Script/Engine.AudioComponent|SetbOverrideAttenuation _returnvalue_11 true)
                          (Rendering|Debug|DrawDebugCircle (Math|Vector|MakeVector _x (.Y (Math|Vector|BreakVector (Variables|Default|GetLastHitPosition))) _z) 1e+01 12 "(R=0.004252,G=1.000000,B=0.000000,A=1.000000)" 1.0 2.5 "0.000000,1.000000,0.000000" "0.000000,0.000000,1.000000"))))))))))))))

(fn ConstructionScript
  (CallFunction|CreateWidget))

(fn GetGameTime
  (return (- (Utilities|Time|GetTimeSeconds) (Variables|Default|GetStartTime))))

(fn GetMoveXDistance
  (return (Math|Float|Absolute(Float) (- (.X (Math|Vector|BreakVector (Transformation|GetWorldLocation (Variables|Default|GetJudge)))) (.X (Math|Vector|BreakVector (Transformation|GetWorldLocation (Variables|Default|GetStart))))))))

(fn GetJudgelinePos
  (return (.X (Math|Vector|BreakVector (Transformation|GetWorldLocation (Variables|Default|GetJudge))))))

(fn GetMoveYDistance
  (bind _miny (Variables|Default|GetMinY))
  (return (- (Variables|Default|GetMaxY) _miny) _miny))

(fn GetPlayerPosition
  (return (Math|Float|NormalizetoRange (.Y (Math|Vector|BreakVector (Transformation|GetActorLocation))) (Variables|Default|GetMinY) (Variables|Default|GetMaxY))))

(fn IsPositionAcceptable
  (params (Normalized%20Pos%20Y :type Float%20%28single-precision%29))
  (bind _positioncorrectionvalue (Variables|Default|GetPositionCorrectionValue))
  (bind _normalized_pos_y (CallFunction|GetPlayerPosition))
  (return (Math|Float|InRange(Float) Normalized%20Pos%20Y (- _normalized_pos_y _positioncorrectionvalue) (+ _normalized_pos_y _positioncorrectionvalue))))

(fn CreateWidget
  (bind _returnvalue (UserInterface|CreateWidget "/Game/Custom/Blueprints/PauseMenu.PauseMenu_C" (Game|GetPlayerController 0)))
  (Variables|Default|SetPauseMenu _returnvalue))

(fn OnContinue
  (Variables|Default|SetisPlaying true)
  (Utilities|Time|SetGlobalTimeDilation 1.0)
  (Variables|Default|SetisPausing false)
  (Widget|SetVisibility (Variables|Default|GetPauseMenu) "Collapsed")
  (Class|AudioComponent|SetPaused (Variables|Default|GetMusic) false)
  (Variables|/Script/Engine.PlayerController|SetbShowMouseCursor (Game|GetPlayerController 0) false))