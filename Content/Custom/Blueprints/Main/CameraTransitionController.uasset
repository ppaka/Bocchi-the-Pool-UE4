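; CameraTransitionController cycles the player's view through an array of target points using keyboard input.
; Each Tick polls Left/A and Right/D on player controller 0 to step an index backward or forward, wrapping at both ends.
; Each step calls SetViewTargetWithBlend on the selected point for a short ease-in-out camera blend with the outgoing view locked.
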(event EventTick
  (params (DeltaSeconds :type Float%20%28single-precision%29))
  (bind _returnvalue (Game|GetPlayerController 0))
  (bind _points (Variables|Default|GetPoints))
  (bind _points_2 (Variables|Default|GetPoints))
  (Utilities|FlowControl|Sequence
    (:then_0
      (if (or (Game|Player|WasInputKeyJustPressed _returnvalue "Left") (Game|Player|WasInputKeyJustPressed _returnvalue "A"))
        (bind _result (Math|Integer|DecrementInt (stale _output_get))
          (:%20%20
            (bind _output_get (Variables|Default|SetIndex _result))
            (if (< _output_get 0)
              (bind _output_get_2 (Variables|Default|SetIndex (- (Utilities|Array|Length _points_2) 1))))
            (Game|Player|SetViewTargetwithBlend _returnvalue (Utilities|Array|Get(acopy) _points_2 _output_get_2) 0.4 "VTBlend_EaseInOut" 3.0 true)))))
    (:then_1
      (if (or (Game|Player|WasInputKeyJustPressed _returnvalue "Right") (Game|Player|WasInputKeyJustPressed _returnvalue "D"))
        (bind _result_2 (Math|Integer|IncrementInt (stale _output_get_3))
          (:%20%20
            (bind _output_get_3 (Variables|Default|SetIndex _result_2))
            (if (>= _output_get_3 (Utilities|Array|Length _points))
              (bind _output_get_4 (Variables|Default|SetIndex 0)))
            (Game|Player|SetViewTargetwithBlend _returnvalue (Utilities|Array|Get(acopy) _points _output_get_4) 0.4 "VTBlend_EaseInOut" 3.0 true)))))))

(fn ConstructionScript)