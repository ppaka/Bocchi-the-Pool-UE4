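; MenuTako is a menu actor that animates in place and opens the LevelSelect level on a mouse click.
; BeginPlay shows the cursor and stores the starting height and yaw as animation baselines.
; Tick replays the Move timeline whenever it finishes, offsetting height and yaw to bob and spin the actor.
; Tick also polls left clicks, accepting any WorldDynamic object under the cursor, not specifically this actor.
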(event EventBeginPlay
  (Variables|/Script/Engine.PlayerController|SetbShowMouseCursor (Game|GetPlayerController 0) true)
  (Variables|Default|SetMoveStartZ (.z (Transformation|GetActorLocation)))
  (Variables|Default|SetRotateStartZ (.yaw (Transformation|GetActorRotation))))

(event EventTick
  (params (DeltaSeconds :type Float%20%28single-precision%29))
  (bind _returnvalue (Game|GetPlayerController 0))
  (bind _returnvalue_2 (Transformation|GetActorLocation))
  (bind _returnvalue_3 (Transformation|GetActorRotation))
  (Utilities|FlowControl|Sequence
    (:then_0
      (if (Game|Player|WasInputKeyJustPressed _returnvalue "LeftMouseButton")
        (if (.ReturnValue (Class|PlayerController|GetHitResultUnderCursorforObjects _returnvalue (Utilities|Array|MakeArray (Utilities|Enum|LiteralenumEObjectTypeQuery "ObjectTypeQuery2")) true))
          (Game|OpenLevel(byName) "LevelSelect"))))
    (:then_1
      (if (Variables|Default|GetAnimEnded)
        (Variables|Default|SetAnimEnded false)
        (bind (_direction _movez _rotatez) (Timeline|Move PlayFromStart)
          (:Update
            (Transformation|SetActorLocationAndRotation (Math|Vector|MakeVector (.x _returnvalue_2) (.y _returnvalue_2) (+ (Variables|Default|GetMoveStartZ) (* _movez 5e+01))) (Math|Rotator|MakeRotator (.roll _returnvalue_3) (.pitch _returnvalue_3) (+ (Variables|Default|GetRotateStartZ) (* _rotatez 7.2e+02))) false true))
          (:Finished
            (Variables|Default|SetAnimEnded true)))))))

(fn ConstructionScript)