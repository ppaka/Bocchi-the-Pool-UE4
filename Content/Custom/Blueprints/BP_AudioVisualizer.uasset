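; Audio spectrum visualizer actor that drives a row of scaled bar actors from a playing sound.
; Init stores the sound's duration and a Constant-Q NRT analysis asset, then spawns the evenly spaced bars, reverses their order and binds to playback percent.
; Each playback update converts percent to time, samples the precomputed normalized channel 0 spectrum and sets each bar's Z scale per band.
; ResetSticks flattens all bars to their base height.
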(event Custom|OnInit_Event
  (params (Audio :type Audio%20Component%20Object%20Reference))
  (bind _returnvalue (Math|Float|MakeLiteralFloat 5e+01))
  (bind _returnvalue_2 (Transformation|GetActorLocation))
  (bind _returnvalue_3 (Class|KismetSystemLibrary|MakeLiteralInteger 47))
  (bind _audioactors (Variables|Default|GetAudioActors))
  (for _index (range 0 _returnvalue_3)
    (bind _returnvalue_4 (Game|SpawnActorfromClass "/Game/Custom/Blueprints/BP_AudioActor.BP_AudioActor_C" (Math|Transform|MakeTransform (Math|Vector|MakeVector (- (* _index _returnvalue) (* (* _returnvalue_3 _returnvalue) 0.5)) (.y _returnvalue_2) (.z _returnvalue_2)) "0, 0, 0" (Math|Vector|MakeVector 0.5 0.1 0.1)) "AlwaysSpawn" 0 0))
    (Utilities|Array|Add _audioactors _returnvalue_4))
  (Utilities|Array|Reverse _audioactors)
  (EventDispatchers|BindEventtoOnAudioPlaybackPercent Audio (delegate Custom|AudioPlayback)))

(event Custom|AudioPlayback
  (params (PlayingSoundWave :type Sound%20Wave%20Object%20Reference) (PlaybackPercent :type Float%20%28single-precision%29))
  (Variables|Default|SetPlayedTime (* PlaybackPercent (Variables|Default|GetDuration)))
  (for (_array_element _array_index) (Class|ConstantQNRT|GetNormalizedChannelConstantQatTime (Variables|Default|GetConstant_Ref) (Variables|Default|GetPlayedTime))
    (Utilities|IsValid (Utilities|Array|Get(acopy) (Variables|Default|GetAudioActors) _array_index)
      (:Is%20Valid
        (Transformation|SetWorldScale3D (Variables|/Game/Custom/Blueprints/BP_AudioActor.BP_AudioActor_C|GetCube (Utilities|Array|Get(acopy) (Variables|Default|GetAudioActors) _array_index)) (Math|Vector|MakeVector 0.5 0.1 (+ (.z (* (Math|Conversions|ToVector(Float) _array_element) 7.5)) 0.1)))))))

(fn ConstructionScript)

(fn Init
  (params (Audio :type Audio%20Component%20Object%20Reference) (ConstantQNRT :type Constant%20QNRT%20Object%20Reference))
  (Variables|Default|SetConstant_Ref ConstantQNRT)
  (Variables|Default|SetDuration (Variables|/Script/Engine.SoundBase|GetDuration (Variables|/Script/Engine.AudioComponent|GetSound Audio)))
  (CallFunction|OnInitEvent Audio))

(fn ResetSticks
  (for _array_element (Variables|Default|GetAudioActors)
    (Transformation|SetWorldScale3D (Variables|/Game/Custom/Blueprints/BP_AudioActor.BP_AudioActor_C|GetCube _array_element) (Math|Vector|MakeVector (.x (Transformation|GetWorldScale (Variables|/Game/Custom/Blueprints/BP_AudioActor.BP_AudioActor_C|GetCube _array_element))) (.y (Transformation|GetWorldScale (Variables|/Game/Custom/Blueprints/BP_AudioActor.BP_AudioActor_C|GetCube _array_element))) 0.1))))