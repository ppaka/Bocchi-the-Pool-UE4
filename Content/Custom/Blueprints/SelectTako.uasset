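; SelectTako is an actor Blueprint that plays a looping bob and spin animation, apparently for an octopus shown in a selection context.
; Tick restarts the Move timeline whenever the previous run has finished, using the AnimEnded flag as a gate.
; Each timeline update teleports the actor, offsetting Z from MoveStartZ and adding yaw to RotateStartZ from the MoveZ and RotateZ tracks.
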(event EventTick
  (params (DeltaSeconds :type Float%20%28single-precision%29))
  (bind _returnvalue (Transformation|GetActorLocation))
  (bind _returnvalue_2 (Transformation|GetActorRotation))
  (if (Variables|Default|GetAnimEnded)
    (Variables|Default|SetAnimEnded false)
    (bind (_direction _movez _rotatez) (Timeline|Move PlayFromStart)
      (:Update
        (Transformation|SetActorLocationAndRotation (Math|Vector|MakeVector (.x _returnvalue) (.y _returnvalue) (+ (Variables|Default|GetMoveStartZ) (* _movez 5.0))) (Math|Rotator|MakeRotator (.roll _returnvalue_2) (.pitch _returnvalue_2) (+ (Variables|Default|GetRotateStartZ) (* _rotatez 3.6e+02))) false true))
      (:Finished
        (Variables|Default|SetAnimEnded true)))))

(fn ConstructionScript)