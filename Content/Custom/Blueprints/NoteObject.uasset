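; NoteObject is a rhythm game note actor that moves relative to the judgeline.
; Each tick it derives X from game time, its start time and Bocchi's duration and travel distance, reaching the judgeline at the start time.
; Y maps the note's data onto Bocchi's Y range, while Z follows the Cube component.
; SetArrowDirection hides both arrows for Touch notes and shows left or right by Direction for Tap and Flick.
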(event EventTick
  (params (DeltaSeconds :type Float%20%28single-precision%29))
  (bind _bocchi (Variables|Default|GetBocchi))
  (bind _notedata (Variables|Default|GetNoteData))
  (bind (_starttime _y) (Utilities|Struct|BreakNoteData _notedata))
  (Utilities|IsValid _bocchi
    (:Is%20Valid
      (bind _x (Default|GetMoveXDistance _bocchi))
      (bind _time (Default|GetGameTime _bocchi))
      (bind _x_2 (Default|GetJudgelinePos _bocchi))
      (bind (_y_distance _min_y) (Default|GetMoveYDistance _bocchi))
      (Transformation|SetActorLocation (Math|Vector|MakeVector (+ _x_2 (* _x (/ (- _time _starttime) (Variables|/Game/Custom/Blueprints/Bocchi.Bocchi_C|GetDuration _bocchi)))) (+ _min_y (* _y_distance _y)) (.Z (Math|Vector|BreakVector (Transformation|GetWorldLocation (Variables|Default|GetCube))))) false true))))

(fn ConstructionScript)

(fn SetArrowDirection
  (bind _notedata (Variables|Default|GetNoteData))
  (bind (_starttime _y _notetype _direction) (Utilities|Struct|BreakNoteData _notedata))
  (switch Utilities|FlowControl|Switch|SwitchonNoteType _notetype
    (:NewEnumerator0
      (Rendering|SetVisibility (Variables|Default|GetLeftArrow) false false)
      (Rendering|SetVisibility (Variables|Default|GetRightArrow) false false))
    (:NewEnumerator1
      (if (<= _direction -1) :!label _label
        (Rendering|SetVisibility (Variables|Default|GetLeftArrow) true false)
        (Rendering|SetVisibility (Variables|Default|GetRightArrow) false false)
        (else
          (Rendering|SetVisibility (Variables|Default|GetLeftArrow) false false)
          (Rendering|SetVisibility (Variables|Default|GetRightArrow) true false))))
    (:NewEnumerator2
      (goto _label))))