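; Game Instance for Bocchi-the-Pool that manages Discord Rich Presence and the persistent save data.
; Init creates the Discord object with an idle presence and loads or creates the BP_SaveData slot, while Shutdown destroys the Discord object.
; Helper functions update presence with an optional timer, write the save, and compute a Unix timestamp in milliseconds.
; The bound Discord result callbacks are effectively empty stubs.
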(event Custom|OnDetailsSet_Event
  (params (StateSetResult :type EDiscordReturnResult%20Enum :default "Ok"))
  ;[0 0.7891 1] Callback delegates
  (switch Utilities|FlowControl|Switch|SwitchonEDiscordReturnResult StateSetResult))

(event Custom|OnLargeImageSet_Event
  (params (StateSetResult :type EDiscordReturnResult%20Enum :default "Ok"))
  ;[0 0.7891 1] Callback delegates
)

(event Custom|OnStateSet_Event
  (params (StateSetResult :type EDiscordReturnResult%20Enum :default "Ok"))
  ;[0 0.7891 1] Callback delegates
)

(event Custom|OnTimerEnd_Event
  (params (StateSetResult :type EDiscordReturnResult%20Enum :default "Ok"))
  ;[0 0.7891 1] Callback delegates
)

(event Custom|OnTimerStart_Event
  (params (StateSetResult :type EDiscordReturnResult%20Enum :default "Ok"))
  ;[0 0.7891 1] Callback delegates
)

(event EventShutdown
  (Class|DiscordObject|DestroyDiscordObject)
  (Variables|Default|SetDiscordObj 0))

(event EventInit
  (bind _returnvalue (Class|DiscordObject|GetDiscordObject))
  (Utilities|FlowControl|Sequence
    (:then_0
      (Utilities|IsValid _returnvalue
        (:Is%20Valid
          _)
        (:Is%20Not%20Valid
          (Class|DiscordObject|CreateDiscordObject "1081347719450349610" false false)))
      (Variables|Default|SetDiscordObj _returnvalue)
      (Utilities|FlowControl|Sequence
        (:then_0
          ;[0 0 0] Optional. You can bind all the available delegates for Discord Object here before calling the main functions.
          (EventDispatchers|AssignOnDetailsSet (Variables|Default|GetDiscordObj) (EventDispatchers|CreateEvent :!event Custom|OnDetailsSet_Event))
          (EventDispatchers|AssignOnLargeImageSet (Variables|Default|GetDiscordObj) (EventDispatchers|CreateEvent :!event Custom|OnLargeImageSet_Event))
          (EventDispatchers|AssignOnStateSet (Variables|Default|GetDiscordObj) (EventDispatchers|CreateEvent :!event Custom|OnStateSet_Event))
          (EventDispatchers|AssignOnTimerEnd (Variables|Default|GetDiscordObj) (EventDispatchers|CreateEvent :!event Custom|OnTimerEnd_Event))
          (EventDispatchers|AssignOnTimerStart (Variables|Default|GetDiscordObj) (EventDispatchers|CreateEvent :!event Custom|OnTimerStart_Event)))
        (:then_1
          (Class|DiscordObject|SetDetails (Variables|Default|GetDiscordObj) "Idle")
          (Class|DiscordObject|SetState (Variables|Default|GetDiscordObj))
          (Class|DiscordObject|SetLargeImage (Variables|Default|GetDiscordObj) "icon"))))
    (:then_1
      (bind _returnvalue_2 (SaveGame|DoesSaveGameExist "Bocchi"))
      (if _returnvalue_2
        (bind _returnvalue_3 (SaveGame|LoadGamefromSlot "Bocchi"))
        (bind _asbp_save_data (Utilities|Casting|CastToBP_SaveData _returnvalue_3))
        (Variables|Default|SetSaveData _asbp_save_data)
        (else
          (bind _returnvalue_4 (SaveGame|CreateSaveGameObject "/Game/Custom/Blueprints/BP_SaveData.BP_SaveData_C"))
          (bind _output_get (Variables|Default|SetSaveData _returnvalue_4))
          (SaveGame|SaveGametoSlot _output_get "Bocchi"))))))

(fn SetPresence
  (params (Details :type String) (State :type String) (StartTimeStamp :type Boolean))
  (bind _discordobj (Variables|Default|GetDiscordObj))
  (Class|DiscordObject|SetDetails _discordobj Details)
  (Class|DiscordObject|SetState _discordobj State)
  (Class|DiscordObject|SetLargeImage _discordobj "icon")
  (Class|DiscordObject|SetLargeImageText _discordobj "Bocchi-the-Pool!")
  (if StartTimeStamp
    (Class|DiscordObject|StartDiscordTimer _discordobj)
    (else
      (Class|DiscordObject|StopDiscordTimer _discordobj))))

(fn GetTimestamp
  (bind _returnvalue (Math|DateTime|UTCNow))
  (bind _returnvalue_2 (Math|DateTime|MakeDateTime 1970 1 1))
  (bind _returnvalue_3 (- _returnvalue _returnvalue_2))
  (return (+ (* (Class|KismetMathLibrary|ToInt64(Integer) (+ (* (Math|Float|Floor (Math|Timespan|GetTotalHours _returnvalue_3)) 3600) (* (Math|Timespan|GetMinutes _returnvalue_3) 60) (Math|Timespan|GetSeconds _returnvalue_3))) 1000) (Class|KismetMathLibrary|ToInt64(Integer) (Class|KismetMathLibrary|GetMilliseconds _returnvalue_3)))))

(fn GameSave
  (SaveGame|SaveGametoSlot (Variables|Default|GetSaveData) "Bocchi"))